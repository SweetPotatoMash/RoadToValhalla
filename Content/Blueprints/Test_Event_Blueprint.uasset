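; Test audio emitter actor that plays its AudioComponent on BeginPlay and applies wall occlusion relative to the first player pawn.
; Tick uses a Delay to throttle updates to UpdateRate, then checks player distance against MaxDistance.
; In range, a WorldStatic multi line trace runs from emitter to player, drawing debug lines.
; Hit count scaled by OcclusionPercent drives the LP_Filter sound parameter, zero when unobstructed.
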(event `self.ReceiveBeginPlay`
  ;[1 1 1] Play Event
  (`FMODAudioComponent.Play` (`self.AudioComponent`))
  (set `self.Player_List` (`GameplayStatics.GetPlayerPawn` 0)))

(event `self.ReceiveTick`
  (params (DeltaSeconds :type "Float (single-precision)"))
  (bind _audiocomponent (`self.AudioComponent`))
  (`KismetSystemLibrary.Delay` (`self.Update_Rate`))
  (bind _returnvalue (`self.GetLocationDifference` (`self.K2_GetActorLocation` (`self.Player_List`)) (`self.K2_GetActorLocation`)))
  (bind _output_get (set `self.Distance` _returnvalue))
  (if (<= _output_get (`self.Max_Distance`))
    (bind (_outhits _returnvalue_2) (`KismetSystemLibrary.LineTraceMultiForObjects` (`self.Audio_Location`) (`self.Player_Location`) (`|MakeArray` "ObjectTypeQuery1" :!type "EObjectTypeQuery Enum") false (`|MakeArray` (`self.Player_List`) :!type "Actor Object Reference") "ForOneFrame"))
    (if _returnvalue_2
      (`FMODAudioComponent.SetParameter` _audiocomponent "LP_Filter" (/ (* (`KismetMathLibrary.Conv_IntToDouble` (`KismetArrayLibrary.Array_Length` _outhits)) (`self.Occlusion_Percent`)) 100.0))
      (else
        (`FMODAudioComponent.SetParameter` _audiocomponent "LP_Filter" 0.0)))))

(fn `GetLocationDifference`
  (params (Player_Location :type "Vector Structure") (Audio_Location :type "Vector Structure"))
  (returns (ReturnValue :type "Float (double-precision)"))
  (bind _output_get (set `self.Player_Location` Player_Location))
  (bind _output_get_2 (set `self.Audio_Location` Audio_Location))
  (return (`KismetMathLibrary.VSize` (- _output_get _output_get_2))))

(fn `UserConstructionScript`)