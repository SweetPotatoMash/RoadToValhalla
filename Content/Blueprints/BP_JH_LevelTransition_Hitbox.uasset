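; BP_JH_LevelTransition_Hitbox is a trigger volume that moves play to another level when an actor overlaps it.
; On overlap it disables that actor's input, without filtering which actor entered, then calls FadeToBlack, which is an empty stub.
; It writes its SpawnLocationIndex into BP_JH_GameInstance's SpawnPointIndex to carry the spawn point across the load, then opens TransitionLevel by object reference.
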(event `self.TransitionHitbox.OnComponentBeginOverlap`
  (params (OverlappedComponent :type "PrimitiveComponent Object Reference") (OtherActor :type "Actor Object Reference") (OtherComp :type "PrimitiveComponent Object Reference") (OtherBodyIndex :type Integer) (bFromSweep :type Boolean) (SweepResult :type "HitResult Structure (by ref)"))
  (`self.LockInputs` OtherActor)
  (`self.FadeToBlack`)
  (`self.SetCorrespondingSpawnPoint`)
  (`GameplayStatics.OpenLevelBySoftObjectPtr` (`self.TransitionLevel`) false))

(fn `FadeToBlack`)

(fn `LockInputs`
  (params (Player :type "Actor Object Reference"))
  (`self.DisableInput` Player null))

(fn `SetCorrespondingSpawnPoint`
  (bind _asbp_jh_game_instance (cast `/Game/Blueprints/BP_JH_GameInstance` (`GameplayStatics.GetGameInstance`)))
  (set `/Game/Blueprints/BP_JH_GameInstance.SpawnPointIndex` (`self.SpawnLocationIndex`) _asbp_jh_game_instance))

(fn `UserConstructionScript`)