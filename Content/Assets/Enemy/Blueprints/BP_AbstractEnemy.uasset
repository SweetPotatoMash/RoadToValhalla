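; BP_AbstractEnemy is an enemy Blueprint, named as an abstract base, that tracks health and an action state.
; AnyDamage subtracts damage from EnemyHealth and clamps it between zero and MaxEnemyHealth.
; Every Tick, SetActionState promotes the queued next state to current, then queues one of two enum values based on whether health is depleted, so state changes lag one update behind.
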(event `self.ReceiveTick`
  (params (DeltaSeconds :type "Float (single-precision)"))
  (`self.SetActionState`))

(event `self.ReceiveAnyDamage`
  (params (Damage :type "Float (single-precision)") (DamageType :type "DamageType Object Reference") (InstigatedBy :type "Controller Object Reference") (DamageCauser :type "Actor Object Reference"))
  (set `self.EnemyHealth` (`KismetMathLibrary.FClamp` (- (`self.EnemyHealth`) Damage) 0.0 (`self.MaxEnemyHealth`))))

(fn `SetActionState`
  (returns (CurrentActionState :type "/Game/Assets/Enemy/Blueprints/E_EnemyState Enum") (NextActionState :type "/Game/Assets/Enemy/Blueprints/E_EnemyState Enum"))
  (bind _output_get (set `self.CurrentActionState` (`self.NextActionState`)))
  (bind _output_get_2 (set `self.NextActionState` (select `bool` (<= (`self.EnemyHealth`) 0.0) :`false` "NewEnumerator0" :`true` "NewEnumerator4" :!type "/Game/Assets/Enemy/Blueprints/E_EnemyState Enum")))
  (return _output_get _output_get_2))

(fn `UserConstructionScript`)