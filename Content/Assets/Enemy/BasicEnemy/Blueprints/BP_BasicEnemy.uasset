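; BP_BasicEnemy is the basic enemy Blueprint, whose only logic of its own here sets its health.
; Its construction script runs the parent's, then copies MaxBasicEnemyHealth from BP_JH_GameInstance into MaxEnemyHealth and sets EnemyHealth to that maximum.
; If the game instance cast fails, neither value is set.
; The event graph holds only disabled placeholder events.
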(fn `UserConstructionScript`
  (`parent.UserConstructionScript`)
  (bind _asbp_jh_game_instance (cast `/Game/Blueprints/BP_JH_GameInstance` (`GameplayStatics.GetGameInstance`)))
  (bind _output_get (set `self.MaxEnemyHealth` (`/Game/Blueprints/BP_JH_GameInstance.MaxBasicEnemyHealth` _asbp_jh_game_instance)))
  (set `self.EnemyHealth` _output_get))