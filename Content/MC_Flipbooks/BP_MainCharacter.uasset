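; Paper2D side-view player character that moves along the Y axis from an input axis and jumps on a button press.
; Each Tick, Animate updates facing from that axis and picks a state by priority: wing jump, airborne, attack, dash by speed threshold, walk, idle.
; State and facing select the left or right flipbook, with attack and wing jump reusing idle and jump animations.
; ResetStates clears the attack and double-jump flags.
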(event `self.ReceiveTick`
  (params (DeltaSeconds :type "Float (single-precision)"))
  (`self.Animate`))

(event `InputAxis|LeftOrRight`
  (params (AxisValue :type "Float (single-precision)"))
  (`self.AddMovementInput` (0.0 -1.0 0.0) AxisValue))

(event `InputAction|Jump`
  (params (Key :type "Key Structure"))
  (:`Pressed`
    (`self.Jump`)))

(fn `Animate`
  (locals (LocalLeftOrRight :type "Float (double-precision)" :default 0.0))
  (bind _returnvalue (`self.GetInputAxisValue`))
  (bind (_animations_idleleft _animations_walkleft _animations_dashleft _animations_jumpleft _animations_idleright _animations_walkright _animations_dashright _animations_jumpright) (break `/Game/MC_Flipbooks/F_MC_Animation` (`self.Animations`)))
  (set `local.LocalLeftOrRight` _returnvalue)
  (if (> _returnvalue 0.0)
    (set `self.FacingRIght` true))
  (if (< (`self.GetInputAxisValue`) 0.0)
    (set `self.FacingRIght` false))
  (set `self.MoveDirection` (select `bool` (`self.DoubleJumping`) :`false` (select `bool` (or (`NavMovementComponent.IsFalling` (`self.CharacterMovement`)) (`NavMovementComponent.IsFlying` (`self.CharacterMovement`))) :`false` (select `bool` (`self.Attacking`) :`false` (select `bool` (> (`KismetMathLibrary.VSize` (`self.GetVelocity`)) (`self.DashThreshold`)) :`false` (select `bool` (> (`KismetMathLibrary.Abs` (`local.LocalLeftOrRight`)) 0.0) :`false` "NewEnumerator0" :`true` "NewEnumerator6" :!type "/Game/MC_Flipbooks/E_MC_Movement Enum") :`true` "NewEnumerator8") :`true` "NewEnumerator12") :`true` "NewEnumerator10") :`true` "NewEnumerator14"))
  (`PaperFlipbookComponent.SetFlipbook` (`self.Sprite`) (select `bool` (`self.FacingRIght`) :`false` (select `/Game/MC_Flipbooks/E_MC_Movement` (`self.MoveDirection`) :`NewEnumerator0` _animations_idleleft :`NewEnumerator6` _animations_walkleft :`NewEnumerator8` _animations_dashleft :`NewEnumerator10` _animations_jumpleft :`NewEnumerator12` _animations_idleleft :`NewEnumerator14` _animations_jumpleft) :`true` (select `/Game/MC_Flipbooks/E_MC_Movement` (`self.MoveDirection`) :`NewEnumerator0` _animations_idleright :`NewEnumerator6` _animations_walkright :`NewEnumerator8` _animations_dashright :`NewEnumerator10` _animations_jumpright :`NewEnumerator12` _animations_idleright :`NewEnumerator14` _animations_jumpright))))

(fn `ResetStates`
  (set `self.Attacking` false)
  (set `self.DoubleJumping` false))

(fn `UserConstructionScript`)