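; BP_MainCharacter is a 2D side-scrolling player character with left/right movement along the world Y axis and jumping.
; Each tick, Animate derives a direction state from the axis input, dash threshold, airborne state and Y velocity.
; That state and current speed select a walk, dash, jump or idle flipbook for the sprite.
; The flipbook updates only while horizontal input is non-zero, and dashing only changes animation here.
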(event `self.ReceiveTick`
  (params (DeltaSeconds :type "Float (single-precision)"))
  (`self.Animate`))

(event `InputAxis|LeftOrRight`
  (params (AxisValue :type "Float (single-precision)"))
  (`self.AddMovementInput` (0.0 -1.0 0.0) AxisValue))

(event `InputAction|Jump`
  (params (Key :type "Key Structure"))
  (:`Pressed`
    (`self.Jump`)))

(fn `Animate`
  (locals (LocalLeftOrRight :type "Float (double-precision)" :default 0.0) (LocalJump :type "Float (double-precision)" :default 0.0))
  (bind (_returnvalue_x _returnvalue_y) (`KismetMathLibrary.BreakVector` (`self.GetVelocity`)))
  (bind (_returnvalue_x_2 _returnvalue_y_2) (`KismetMathLibrary.BreakVector` (`self.GetVelocity`)))
  (bind (_animations_idleleft _animations_walkleft _animations_idleright _animations_walkright _animations_jumpleft _animations_jumpright _animations_dashleft _animations_dashright) (break `/Game/F_MC_Animation` (`self.Animations`)))
  (set `local.LocalLeftOrRight` (`self.GetInputAxisValue`))
  (if (!= (`local.LocalLeftOrRight`) 0.0)
    (set `self.MoveDirection` (select `bool` (and (or (`NavMovementComponent.IsFalling` (`self.CharacterMovement`)) (`NavMovementComponent.IsFlying` (`self.CharacterMovement`))) (< _returnvalue_y_2 0.0)) :`false` (select `bool` (and (or (`NavMovementComponent.IsFalling` (`self.CharacterMovement`)) (`NavMovementComponent.IsFlying` (`self.CharacterMovement`))) (> _returnvalue_y 0.0)) :`false` (select `bool` (> (`local.LocalLeftOrRight`) (`self.DashThreshold`)) :`false` (select `bool` (< (`local.LocalLeftOrRight`) (* (`self.DashThreshold`) -1.0)) :`false` (select `bool` (> (`local.LocalLeftOrRight`) 0.0) :`false` "NewEnumerator0" :`true` "NewEnumerator1" :!type "/Game/E_MC_Movement Enum") :`true` "NewEnumerator3") :`true` "NewEnumerator4") :`true` "NewEnumerator2") :`true` "NewEnumerator5"))
    (`PaperFlipbookComponent.SetFlipbook` (`self.Sprite`) (select `bool` (> (`KismetMathLibrary.VSize` (`self.GetVelocity`)) 0.0) :`false` (select `/Game/E_MC_Movement` (`self.MoveDirection`) :`NewEnumerator0` _animations_idleleft :`NewEnumerator1` _animations_idleright :`NewEnumerator2` _animations_jumpleft :`NewEnumerator5` _animations_jumpright :`NewEnumerator3` _animations_idleleft :`NewEnumerator4` _animations_idleright) :`true` (select `/Game/E_MC_Movement` (`self.MoveDirection`) :`NewEnumerator0` _animations_walkleft :`NewEnumerator1` _animations_walkright :`NewEnumerator2` _animations_jumpleft :`NewEnumerator5` _animations_jumpright :`NewEnumerator3` _animations_dashleft :`NewEnumerator4` _animations_dashright)))))

(fn `UserConstructionScript`)