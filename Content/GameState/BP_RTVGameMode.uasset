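; Game mode that handles player respawning and combat-reactive level music.
; Each tick after music setup, it scans the game instance's level enemies and sets the music event's "Transition" parameter by whether any is chasing.
; Respawns destroy the player pawn, spawn and possess a new one at the spawn location, optionally after a delay, using the starting spawn on game over.
; It also provides spawn-point setters and a camera fade from black.
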(event `SetLevelMusic`
  (params (LevelMusic :type "FMODEventInstance Structure"))
  (set `self.LevelMusic` LevelMusic)
  (set `self.SetupComplete` true))

(event `self.ReceiveBeginPlay`
  (bind _asbp_jh_game_instance (cast `/Game/GameState/BP_JH_GameInstance` (`GameplayStatics.GetGameInstance`)))
  (set `self.GameInstance` _asbp_jh_game_instance))

(event `self.ReceiveTick`
  (params (DeltaSeconds :type "Float (single-precision)"))
  (bind _levelmusic (`self.LevelMusic`))
  (bind _levelenemies (`/Game/GameState/BP_JH_GameInstance.LevelEnemies` (`self.GameInstance`)))
  (if (`self.SetupComplete`)
    (if (> (`KismetArrayLibrary.Array_Length` _levelenemies) 0)
      (for _array_element _levelenemies
        (`/Engine/EditorBlueprintResources/StandardMacros.IsValid` _array_element
          (:`Is Valid`
            (if (`/Game/Actors/Enemy/Blueprints/BP_AbstractEnemy.Chasing` _array_element)
              (set `self.IsPlayerInCombat` true)
              (break)))))
      (if (`self.IsPlayerInCombat`)
        (`FMODBlueprintStatics.EventInstanceSetParameter` _levelmusic "Transition" 2.0)
        (else
          (`FMODBlueprintStatics.EventInstanceSetParameter` _levelmusic "Transition")))
      (set `self.IsPlayerInCombat` false))))

(event `SpawnPlayer`
  (params (RespawnType :type "/Game/Actors/Player/Character/Blueprints/RespawnTypes Enum" :default "NewEnumerator0"))
  (bind _returnvalue (`GameplayStatics.GetPlayerController` 0))
  (bind _player (`self.Player`))
  (if (`KismetSystemLibrary.IsValid` _player)
    (`self.K2_DestroyActor` _player))
  (set `/Game/GameState/BP_JH_GameInstance.RespawnType` RespawnType (`self.GameInstance`))
  (bind _returnvalue_2 (`|SpawnActorFromClass` "/Game/Actors/Player/Character/Blueprints/ND_PlayerSprite.ND_PlayerSprite_C" (`KismetMathLibrary.Conv_VectorToTransform` (`self.SpawnLocation`)) "AlwaysSpawn" "OverrideRootScale" null null))
  (bind _output_get (set `self.Player` _returnvalue_2))
  (`Controller.Possess` _returnvalue _output_get)
  (`self.EnableInput` _output_get _returnvalue))

(event `Respawn`
  (`self.BeginRespawnPlayer` false))

(event `RespawnWithDelay`
  (`self.BeginRespawnPlayer` true))

(event `DelayRespawn`
  (`KismetSystemLibrary.Delay` 2.0)
  (`self.SpawnPlayer` "NewEnumerator0"))

(fn `BeginRespawnPlayer`
  (params (IsDelayed :type Boolean))
  (if (`self.GameOver`)
    (set `self.SpawnLocation` (`KismetMathLibrary.TransformLocation` (`self.StartingSpawn`))))
  (if IsDelayed
    (`self.DelayRespawn`)
    (else
      (`self.SpawnPlayer` "NewEnumerator0"))))

(fn `FadeFromBlack`
  (`GameplayStatics.SetGamePaused` true)
  (`PlayerCameraManager.StartCameraFade` :`self` (`PlayerController.PlayerCameraManager` (`GameplayStatics.GetPlayerController` 0)) :`FromAlpha` 1.0 :`Duration` 1.0)
  (`GameplayStatics.SetGamePaused` false))

(fn `Finish Respawn Player`
  (params (DestroyedActor :type "Actor Object Reference")))

(fn `SetSpawnAs`
  (params (RespawnPoint :type "/Game/Enviornment/Blueprints/BP_JH_RespawnCheckpoint Object Reference") (GameMode :type "/Game/GameState/BP_RTVGameMode Object Reference"))
  (`/Game/Enviornment/Blueprints/BP_JH_RespawnCheckpoint.SetSpawnToThisLocation` RespawnPoint GameMode))

(fn `SetStartingSpawn`
  (params (SpawnLocation :type "Vector Structure"))
  (bind _output_get (set `self.SpawnLocation` SpawnLocation))
  (set `self.StartingSpawn` (`KismetMathLibrary.Conv_VectorToTransform` _output_get)))

(fn `UserConstructionScript`)