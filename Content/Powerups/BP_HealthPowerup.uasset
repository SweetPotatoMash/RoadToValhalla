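; Health pickup that restores health to the player sprite on contact and then removes itself.
; An overlap on its Collision component that casts to ND_PlayerSprite triggers UpdateStats, then destroys the actor.
; UpdateStats adds HealthAmount to the player pawn's PlayerHealth without clamping, then copies the new total into BP_JH_GameInstance.
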(event `self.Collision.OnComponentBeginOverlap`
  (params (OverlappedComponent :type "PrimitiveComponent Object Reference") (OtherActor :type "Actor Object Reference") (OtherComp :type "PrimitiveComponent Object Reference") (OtherBodyIndex :type Integer) (bFromSweep :type Boolean) (SweepResult :type "HitResult Structure (by ref)"))
  (cast `/Game/Actors/Player/Character/Blueprints/ND_PlayerSprite` OtherActor)
  (`self.UpdateStats`)
  (`self.K2_DestroyActor`))

(fn `UpdateStats`
  (bind _asnd_player_sprite (cast `/Game/Actors/Player/Character/Blueprints/ND_PlayerSprite` (`GameplayStatics.GetPlayerPawn` 0)))
  (bind _output_get (set `/Game/Actors/Player/Character/Blueprints/ND_PlayerSprite.PlayerHealth` (+ (`/Game/Actors/Player/Character/Blueprints/ND_PlayerSprite.PlayerHealth` _asnd_player_sprite) (`self.HealthAmount`)) _asnd_player_sprite))
  (bind _asbp_jh_game_instance (cast `/Game/GameState/BP_JH_GameInstance` (`GameplayStatics.GetGameInstance`)))
  (set `/Game/GameState/BP_JH_GameInstance.PlayerHealh` _output_get _asbp_jh_game_instance))

(fn `UserConstructionScript`)