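; Respawn checkpoint actor that moves the player's respawn point when the player reaches it.
; On BeginPlay it caches the world location of its CheckpointHitbox component.
; When an actor of exactly the ND_PlayerSprite class overlaps the hitbox, it writes that cached location to SpawnLocation on BP_RTVGameMode, leaving the respawn itself to code outside this Blueprint.
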(event `self.ReceiveBeginPlay`
  (set `self.LocationOfSpawn` (`SceneComponent.K2_GetComponentLocation` (`self.CheckpointHitbox`))))

(event `self.CheckpointHitbox.OnComponentBeginOverlap`
  (params (OverlappedComponent :type "PrimitiveComponent Object Reference") (OtherActor :type "Actor Object Reference") (OtherComp :type "PrimitiveComponent Object Reference") (OtherBodyIndex :type Integer) (bFromSweep :type Boolean) (SweepResult :type "HitResult Structure (by ref)"))
  (if (== (`GameplayStatics.GetObjectClass` OtherActor) "/Game/Actors/Player/Character/Blueprints/ND_PlayerSprite.ND_PlayerSprite_C")
    (bind _asbp_rtvgame_mode (cast `/Game/GameState/BP_RTVGameMode` (`GameplayStatics.GetGameMode`)))
    (`self.SetSpawnToThisLocation` _asbp_rtvgame_mode)))

(fn `SetSpawnToThisLocation`
  (params (GameMode :type "/Game/GameState/BP_RTVGameMode Object Reference"))
  (set `/Game/GameState/BP_RTVGameMode.SpawnLocation` (`self.LocationOfSpawn`) GameMode))

(fn `UserConstructionScript`)