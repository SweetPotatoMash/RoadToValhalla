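; BP_JH_LevelTransition_Hitbox is a trigger that moves the player to another level when ND_PlayerSprite overlaps it.
; On overlap it disables player input and stores its SpawnLocationIndex as the spawn point index in BP_JH_GameInstance, redundantly setting it twice.
; It then opens the level at SpawnLevelIndex in that game instance's Levels array.
; FadeToBlack is called but is an empty stub.
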(event `self.TransitionHitbox.OnComponentBeginOverlap`
  (params (OverlappedComponent :type "PrimitiveComponent Object Reference") (OtherActor :type "Actor Object Reference") (OtherComp :type "PrimitiveComponent Object Reference") (OtherBodyIndex :type Integer) (bFromSweep :type Boolean) (SweepResult :type "HitResult Structure (by ref)"))
  (if (== (`GameplayStatics.GetObjectClass` OtherActor) "/Game/Actors/Player/Character/Blueprints/ND_PlayerSprite.ND_PlayerSprite_C")
    (`self.LockInputs` OtherActor)
    (`self.FadeToBlack`)
    (`self.SetCorrespondingSpawnPoint`)
    (bind _asbp_jh_game_instance (cast `/Game/GameState/BP_JH_GameInstance` (`GameplayStatics.GetGameInstance`)))
    (set `/Game/GameState/BP_JH_GameInstance.SpawnPointIndex` (`self.SpawnLocationIndex`) _asbp_jh_game_instance)
    (`GameplayStatics.OpenLevelBySoftObjectPtr` (`|GetArrayItem` (`/Game/GameState/BP_JH_GameInstance.Levels` _asbp_jh_game_instance) (`self.SpawnLevelIndex`)))))

(fn `FadeToBlack`)

(fn `LockInputs`
  (params (Player :type "Actor Object Reference"))
  (`self.DisableInput` Player (`GameplayStatics.GetPlayerController` 0)))

(fn `SetCorrespondingSpawnPoint`
  (bind _asbp_jh_game_instance (cast `/Game/GameState/BP_JH_GameInstance` (`GameplayStatics.GetGameInstance`)))
  (set `/Game/GameState/BP_JH_GameInstance.SpawnPointIndex` (`self.SpawnLocationIndex`) _asbp_jh_game_instance))

(fn `UserConstructionScript`)