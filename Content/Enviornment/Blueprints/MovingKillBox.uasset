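; Moving hazard that deals damage equal to max health to any ND_PlayerSprite overlapping it.
; The construction script turns PathType, Radius and Offset into straight or circular paths in the Y-Z plane, outlined by splines.
; Tick advances Alpha by a per-frame step without delta time, driving endpoint lerps or sine/cosine orbits rather than following the splines.
; Linear paths pause for EndPause at each end before reversing; circles zero that delay.
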(event `self.ReceiveBeginPlay`)

(event `self.ReceiveTick`
  (params (DeltaSeconds :type "Float (single-precision)"))
  (bind (_control1_x _control1_y _control1_z) (`KismetMathLibrary.BreakVector` (`self.Control1`)))
  (`self.UpdateAlpha`)
  (if (`self.IsCircular`)
    ;[1 1 1] Circular Path
    (`self.K2_SetActorLocation` (`KismetMathLibrary.MakeVector` _control1_x (`self.ParametricY` _control1_y) (`self.ParametricZ` _control1_z)) true)
    (else
      ;[1 1 1] Linear Path
      (if (`self.ReachedControl1`)
        (`self.MoveToControl1`)
        (else
          (`self.MoveToControl2`))))))

(event `Pause`
  (`KismetSystemLibrary.Delay` (`self.EndPause`))
  (set `self.Paused?` false))

(event `self.ReceiveActorBeginOverlap`
  (params (OtherActor :type "Actor Object Reference"))
  (bind _asnd_player_sprite (cast `/Game/Actors/Player/Character/Blueprints/ND_PlayerSprite` OtherActor))
  (`GameplayStatics.ApplyDamage` _asnd_player_sprite (`/Game/Actors/Player/Character/Blueprints/ND_PlayerSprite.MaxPlayerHealth` _asnd_player_sprite)))

(fn `DrawCircle`
  (locals (KillLocalSpline :type "SplineComponent Object Reference"))
  (bind (_control1_x _control1_y _control1_z) (`KismetMathLibrary.BreakVector` (`self.Control1`)))
  (bind (_control1_x_2 _control1_y_2 _control1_z_2) (`KismetMathLibrary.BreakVector` (`self.Control1`)))
  (bind (_control1_x_3 _control1_y_3 _control1_z_3) (`KismetMathLibrary.BreakVector` (`self.Control1`)))
  (bind (_control1_x_4 _control1_y_4 _control1_z_4) (`KismetMathLibrary.BreakVector` (`self.Control1`)))
  (bind _returnvalue (`AddComponent|NODE_AddSplineComponent-0`))
  (bind _output_get (set `local.KillLocalSpline` _returnvalue))
  (`SplineComponent.SetLocationAtSplinePoint` _output_get 0 (`KismetMathLibrary.MakeVector` _control1_x_2 (- _control1_y_2 (`self.Radius`)) _control1_z_2) "World" true)
  (`SplineComponent.SetLocationAtSplinePoint` (`local.KillLocalSpline`) 1 (`KismetMathLibrary.MakeVector` _control1_x_3 _control1_y_3 (+ _control1_z_3 (`self.Radius`))) "World" true)
  (`SplineComponent.AddSplinePoint` (`local.KillLocalSpline`) (`KismetMathLibrary.MakeVector` _control1_x_4 (+ _control1_y_4 (`self.Radius`)) _control1_z_4) "World" true)
  (`SplineComponent.AddSplinePoint` (`local.KillLocalSpline`) (`KismetMathLibrary.MakeVector` _control1_x _control1_y (- _control1_z (`self.Radius`))) "World" true)
  (`SplineComponent.SetTangentAtSplinePoint` (`local.KillLocalSpline`) 0 (`KismetMathLibrary.MakeVector` 0.0 0.0 (* (`self.Radius`) 1.66)) "World" true)
  (`SplineComponent.SetTangentAtSplinePoint` (`local.KillLocalSpline`) 1 (`KismetMathLibrary.MakeVector` 0.0 (* (`self.Radius`) 1.66)) "World" true)
  (`SplineComponent.SetTangentAtSplinePoint` (`local.KillLocalSpline`) 2 (`KismetMathLibrary.MakeVector` 0.0 0.0 (* (`self.Radius`) -1.66)) "World" true)
  (`SplineComponent.SetTangentAtSplinePoint` (`local.KillLocalSpline`) 3 (`KismetMathLibrary.MakeVector` 0.0 (* (`self.Radius`) -1.66)) "World" true)
  (`SplineComponent.SetClosedLoop` (`local.KillLocalSpline`) true true)
  (`SceneComponent.SetVisibility` (`self.Spline`) false false))

(fn `GetRadian`
  (returns (Angle :type "Float (double-precision)"))
  (bind _returnvalue (* (`KismetMathLibrary.MultiplyByPi` (`self.Alpha`)) 2.0))
  (if (`self.Clockwise?`)
    (return _returnvalue)
    (else
      (return (* _returnvalue -1.0)))))

(fn `SetControlDistance`
  (params (x :type "Float (double-precision)") (y :type "Float (double-precision)") (z :type "Float (double-precision)"))
  (bind _returnvalue (`self.K2_GetActorLocation`))
  (set `self.Control1` (+ _returnvalue (`KismetMathLibrary.MakeVector` x y z)))
  (set `self.Control2` (- _returnvalue (`KismetMathLibrary.MakeVector` x y z)))
  (`self.SwapControls`)
  (`SplineComponent.SetLocationAtSplinePoint` (`self.Spline`) 0 (`self.Control1`) "World" true)
  (`SplineComponent.SetLocationAtSplinePoint` (`self.Spline`) 1 (`self.Control2`) "World" true))

(fn `SwapControls`
  (locals (Temp :type "Vector Structure" :default (0.0 0.0 0.0)))
  (if (`self.SwapControls?`)
    (set `local.Temp` (`self.Control1`))
    (set `self.Control1` (`self.Control2`))
    (set `self.Control2` (`local.Temp`))))

(fn `UpdateAlpha`
  (if (`self.Paused?`)
    _
    (elif (< (`self.Alpha`) 1.0)
      (set `self.Alpha` (+ (`self.Alpha`) (`self.TrueSpeed`)))
      (else
        (set `self.Alpha` 0.0)
        (set `self.Paused?` true)
        (`self.Pause`)))))

(fn `UserConstructionScript`
  (bind _radius (`self.Radius`))
  (bind _radius_2 (`self.Radius`))
  (set `self.TrueSpeed` (* (`self.TrueSpeed`) (`self.Speed`)))
  (set `self.Alpha` (`self.Offset`))
  (switch `/Game/Enviornment/Blueprints/MovingPlatformEnum` (`self.PathType`)
    (:`NewEnumerator0`
      (`self.SetControlDistance` 0.0 0.0 (`self.Radius`)))
    (:`NewEnumerator1`
      (`self.SetControlDistance` 0.0 (* (`self.Radius`) -1.0)))
    (:`NewEnumerator2`
      (set `self.Control1` (`self.K2_GetActorLocation`))
      (set `self.EndPause` 0.0)
      (set `self.IsCircular` true)
      (`self.DrawCircle`))
    (:`NewEnumerator3`
      (`self.SetControlDistance` 0.0 _radius_2 _radius_2))
    (:`NewEnumerator4`
      (`self.SetControlDistance` 0.0 (* _radius -1.0) _radius))))