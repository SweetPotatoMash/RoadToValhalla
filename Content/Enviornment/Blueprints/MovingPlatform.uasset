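; Moving platform actor that travels back and forth along a vertical, horizontal or diagonal line, or around a circle in the YZ plane.
; The construction script derives two endpoints or a circle centre from the placed location, path type and radius, with an optional endpoint swap.
; Tick advances a normalized Alpha, pausing at the end of each linear leg.
; Alpha drives swept moves via vector lerp or sine/cosine orbit.
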(event `self.ReceiveBeginPlay`)

(event `self.ReceiveTick`
  (params (DeltaSeconds :type "Float (single-precision)"))
  (bind (_control1_x _control1_y _control1_z) (`KismetMathLibrary.BreakVector` (`self.Control1`)))
  (`self.UpdateAlpha`)
  (if (`self.IsCircular`)
    ;[1 1 1] Circular Path
    (`self.K2_SetActorLocation` (`KismetMathLibrary.MakeVector` _control1_x (`self.ParametricY` _control1_y) (`self.ParametricZ` _control1_z)) true)
    (else
      ;[1 1 1] Linear Path
      (if (`self.ReachedControl1`)
        (`self.MoveToControl1`)
        (else
          (`self.MoveToControl2`))))))

(event `Pause`
  (`KismetSystemLibrary.Delay` (`self.EndPause`))
  (set `self.Paused?` false))

(fn `GetRadian`
  (returns (Angle :type "Float (double-precision)"))
  (bind _returnvalue (* (`KismetMathLibrary.MultiplyByPi` (`self.Alpha`)) 2.0))
  (if (`self.Clockwise?`)
    (return _returnvalue)
    (else
      (return (* _returnvalue -1.0)))))

(fn `SetControlDistance`
  (params (x :type "Float (double-precision)") (y :type "Float (double-precision)") (z :type "Float (double-precision)"))
  (bind _returnvalue (`self.K2_GetActorLocation`))
  (set `self.Control1` (+ _returnvalue (`KismetMathLibrary.MakeVector` x y z)))
  (set `self.Control2` (- _returnvalue (`KismetMathLibrary.MakeVector` x y z)))
  (`self.SwapControls`))

(fn `SwapControls`
  (locals (Temp :type "Vector Structure" :default (0.0 0.0 0.0)))
  (if (`self.SwapControls?`)
    (set `local.Temp` (`self.Control1`))
    (set `self.Control1` (`self.Control2`))
    (set `self.Control2` (`local.Temp`))))

(fn `UpdateAlpha`
  (if (`self.Paused?`)
    _
    (elif (< (`self.Alpha`) 1.0)
      (set `self.Alpha` (+ (`self.Alpha`) (`self.TrueSpeed`)))
      (else
        (set `self.Alpha` 0.0)
        (set `self.Paused?` true)
        (`self.Pause`)))))

(fn `UserConstructionScript`
  (bind _radius (`self.Radius`))
  (bind _radius_2 (`self.Radius`))
  (set `self.TrueSpeed` (* (`self.TrueSpeed`) (`self.Speed`)))
  (set `self.Alpha` (`self.Offset`))
  (switch `/Game/Enviornment/Blueprints/MovingPlatformEnum` (`self.PathType`)
    (:`NewEnumerator0`
      (`self.SetControlDistance` 0.0 0.0 (`self.Radius`)))
    (:`NewEnumerator1`
      (`self.SetControlDistance` 0.0 (* (`self.Radius`) -1.0)))
    (:`NewEnumerator2`
      (set `self.Control1` (`self.K2_GetActorLocation`))
      (set `self.EndPause` 0.0)
      (set `self.IsCircular` true))
    (:`NewEnumerator3`
      (`self.SetControlDistance` 0.0 _radius_2 _radius_2))
    (:`NewEnumerator4`
      (`self.SetControlDistance` 0.0 (* _radius -1.0) _radius))))