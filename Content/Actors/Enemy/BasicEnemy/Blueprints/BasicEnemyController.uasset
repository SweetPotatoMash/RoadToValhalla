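; AI controller for 2D Paper enemies that runs either a lunge or basic behavior tree, chosen by pawn class.
; Each tick it writes player death and target state to the Blackboard, acquiring the player when near and dropping it beyond a larger radius.
; Walk speed rises on acquisition; losing the target stops movement, clears chasing and slows the enemy.
; A lunge cooldown event disables the CanLunge key for a short delay.
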(event `self.ReceiveTick`
  (params (DeltaSeconds :type "Float (single-precision)"))
  (bind _blackboard (`self.Blackboard`))
  (bind _aspaper_character (cast `PaperCharacter` (`self.K2_GetPawn`)))
  (bind _asnd_player_sprite (cast `/Game/Actors/Player/Character/Blueprints/ND_PlayerSprite` (`GameplayStatics.GetPlayerCharacter` 0)))
  (if (`/Game/Actors/Player/Character/Blueprints/ND_PlayerSprite.IsDead` _asnd_player_sprite)
    (`BlackboardComponent.SetValueAsBool` (`self.Blackboard`) "IsPlayerDead" true)
    (bind _sprite (`PaperCharacter.Sprite` _aspaper_character))
    (bind _sprite_2 (`PaperCharacter.Sprite` _asnd_player_sprite))
    (if (>= (`KismetMathLibrary.VSize` (- (`SceneComponent.K2_GetComponentLocation` _sprite) (`SceneComponent.K2_GetComponentLocation` _sprite_2))) 800.0) :!label _label
      (`BlackboardComponent.SetValueAsObject` _blackboard "TargetedActor" null)
      (`BlackboardComponent.SetValueAsBool` _blackboard "HasTarget" false)
      (bind _asbp_abstract_enemy (cast `/Game/Actors/Enemy/Blueprints/BP_AbstractEnemy` (`self.K2_GetPawn`)))
      (bind _charactermovement (`Character.CharacterMovement` _asbp_abstract_enemy))
      (`NavMovementComponent.StopActiveMovement` _charactermovement)
      (set `/Game/Actors/Enemy/Blueprints/BP_AbstractEnemy.Chasing` false _asbp_abstract_enemy)
      (set `CharacterMovementComponent.MaxWalkSpeed` 150.0 _charactermovement))
    (else
      (`BlackboardComponent.SetValueAsBool` (`self.Blackboard`) "IsPlayerDead" false)
      (if (`BlackboardComponent.GetValueAsBool` (`self.Blackboard`) "HasTarget")
        (goto _label)
        (elif (<= (`KismetMathLibrary.VSize` (- (`SceneComponent.K2_GetComponentLocation` _sprite) (`SceneComponent.K2_GetComponentLocation` _sprite_2))) 400.0)
          (`BlackboardComponent.SetValueAsObject` (`self.Blackboard`) "TargetedActor" (`GameplayStatics.GetPlayerCharacter` 0))
          (bind _asbp_abstract_enemy_2 (cast `/Game/Actors/Enemy/Blueprints/BP_AbstractEnemy` (`self.K2_GetPawn`)))
          (set `CharacterMovementComponent.MaxWalkSpeed` 300.0 (`Character.CharacterMovement` _asbp_abstract_enemy_2)))))))

(event `self.ReceiveBeginPlay`
  (bind _blackboard (`self.Blackboard`))
  (`self.RunBehaviorTree` (select `bool` (== (`GameplayStatics.GetObjectClass` (`self.K2_GetPawn`)) null) :`false` "/Game/Actors/Enemy/BasicEnemy/Blueprints/BasicEnemyBehavior.BasicEnemyBehavior" :`true` "/Game/Actors/Enemy/BasicEnemy/Blueprints/LungeEnemyBehavior.LungeEnemyBehavior" :!type "BehaviorTree Object Reference"))
  (`BlackboardComponent.SetValueAsBool` _blackboard "CanLunge" true)
  (`BlackboardComponent.SetValueAsBool` _blackboard "HasTarget" false))

(event `LungeCooldown`
  (`BlackboardComponent.SetValueAsBool` (`self.Blackboard`) "CanLunge" false)
  (`KismetSystemLibrary.Delay` 3.0)
  (`BlackboardComponent.SetValueAsBool` (`self.Blackboard`) "CanLunge" true))

(fn `UserConstructionScript`)