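; BP_BasicEnemy is a 2D flipbook enemy that attacks, takes knockback and can grant mana to the player.
; BeginPlay sets combat stats, reading max health from the game instance.
; Tick handles death, derives state and left/right facing from Y velocity for Animate, and times attacks to flipbook frame 1.
; Damage knocks it away from the player, awarding mana to special-equipped players for basic attacks at zero health.
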(event `self.ReceiveBeginPlay`
  (`parent.ReceiveBeginPlay`)
  (bind _asbp_jh_game_instance (cast `/Game/GameState/BP_JH_GameInstance` (`GameplayStatics.GetGameInstance`)))
  (bind _output_get (set `self.MaxEnemyHealth` (`/Game/GameState/BP_JH_GameInstance.MaxBasicEnemyHealth` _asbp_jh_game_instance)))
  (set `self.EnemyHealth` _output_get)
  (set `self.AttackRange` 50.0)
  (set `self.BasicAttackDamage` (`self.BasicEnemyAttackDamage`))
  (set `self.DamagedDuration` 0.7)
  (set `self.ManaValue` 20.0))

(event `self.ReceiveTick`
  (params (DeltaSeconds :type "Float (single-precision)"))
  (bind (_returnvalue_x _returnvalue_y) (`KismetMathLibrary.BreakVector` (`self.GetVelocity`)))
  (bind _nextdirection (`self.NextDirection`))
  (`parent.ReceiveTick` DeltaSeconds)
  (if (`|EnumEquality` (`self.NextActionState`) "NewEnumerator4")
    (if (not (`self.Dead`))
      (`self.Died`))
    (else
      (if (and (`self.Attacking`) (== (`PaperFlipbookComponent.GetPlaybackPositionInFrames` (`self.Sprite`)) 1))
        (if (== (`self.AttackCooldown`) 0.0)
          (set `self.HitDetected` false)
          (`self.Attack`))
        (set `self.AttackCooldown` (+ (`self.AttackCooldown`) DeltaSeconds))
        (else
          (set `self.AttackCooldown` 0.0)))
      (bind (_currentactionstate _nextactionstate) (`self.SetActionState` _returnvalue_y))
      (bind _nextdirection_2 (`self.GetDirection` (* _returnvalue_y -1.0) 0.0 _nextdirection false _nextdirection))
      (bind _output_get (set `self.NextDirection` _nextdirection_2))
      (if (`self.RecievingDamage`)
        (`self.Animate` (`self.KnockbackFacingDirection`) _nextactionstate)
        (else
          (`self.Animate` _output_get _nextactionstate))))))

(event `Damage`
  (params (DamageCauser :type "Actor Object Reference") (IsBasicAttack :type Boolean))
  (bind _asnd_player_sprite (cast `/Game/Actors/Player/Character/Blueprints/ND_PlayerSprite` DamageCauser))
  (if (and (== (`self.EnemyHealth`) 0.0) IsBasicAttack (`/Game/Actors/Player/Character/Blueprints/ND_PlayerSprite.HasSpecial` _asnd_player_sprite))
    (`/Game/Actors/Player/Character/Blueprints/ND_PlayerSprite.AddMana` _asnd_player_sprite (`self.ManaValue`)))
  (bind _direction (`self.GetDirectionOppositePlayer` _asnd_player_sprite))
  (bind _output_get (set `self.KnockbackFacingDirection` _direction))
  (set `self.RecievingDamage` true)
  (`self.DamageKnockback` _output_get 4.5)
  (`self.DamagedCooldown`))

(fn `Animate`
  (params (NextDirection :type "/Game/Actors/Player/Character/Blueprints/ND_PlayerDirection Enum" :default "NewEnumerator0") (NextActionState :type "/Game/Actors/Enemy/Blueprints/E_EnemyState Enum" :default "NewEnumerator0"))
  (locals (LocalNextDirection :type "/Game/Actors/Player/Character/Blueprints/ND_PlayerDirection Enum") (LocalNextActionState :type "/Game/Actors/Enemy/Blueprints/E_EnemyState Enum" :default "NewEnumerator0"))
  (bind (_basicenemyanimation_idleright _basicenemyanimation_idleleft _basicenemyanimation_walkingright _basicenemyanimation_walkingleft _basicenemyanimation_alertedright _basicenemyanimation_alertedleft _basicenemyanimation_attackright _basicenemyanimation_attackleft) (break `/Game/Actors/Enemy/BasicEnemy/Blueprints/BasicEnemyAnims` (`self.BasicEnemyAnimation`)))
  (set `local.LocalNextDirection` NextDirection)
  (set `local.LocalNextActionState` NextActionState)
  (`PaperFlipbookComponent.SetFlipbook` (`self.Sprite`) (select `/Game/Actors/Enemy/Blueprints/E_EnemyState` (`local.LocalNextActionState`) :`NewEnumerator0` (select `/Game/Actors/Player/Character/Blueprints/ND_PlayerDirection` (`local.LocalNextDirection`) :`NewEnumerator0` _basicenemyanimation_idleright :`NewEnumerator1` _basicenemyanimation_idleleft) :`NewEnumerator1` (select `/Game/Actors/Player/Character/Blueprints/ND_PlayerDirection` (`local.LocalNextDirection`) :`NewEnumerator0` _basicenemyanimation_walkingright :`NewEnumerator1` _basicenemyanimation_walkingleft) :`NewEnumerator2` (select `/Game/Actors/Player/Character/Blueprints/ND_PlayerDirection` (`local.LocalNextDirection`) :`NewEnumerator0` _basicenemyanimation_attackright :`NewEnumerator1` _basicenemyanimation_attackleft) :`NewEnumerator3` (select `/Game/Actors/Player/Character/Blueprints/ND_PlayerDirection` (`local.LocalNextDirection`) :`NewEnumerator0` _basicenemyanimation_alertedright :`NewEnumerator1` _basicenemyanimation_alertedleft))))

(fn `UserConstructionScript`
  (`parent.UserConstructionScript`))