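; Base enemy actor for a sprite-based game that chases, attacks and reacts to damage.
; While chasing and undamaged, Tick moves it along Y toward the blackboard's TargetedActor, setting Attacking on arrival.
; SetActionState derives action states by priority from health, alert, attack and velocity, alongside a helper for facing opposite the target.
; BeginPlay writes self into the last Enemies slot; OnDamaged forwards damage by casting self to child BP_BasicEnemy.
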(event `self.ReceiveBeginPlay`
  (bind _enemies (`self.Enemies`))
  (`KismetArrayLibrary.Array_Set` _enemies (`KismetArrayLibrary.Array_LastIndex` _enemies) self true))

(event `self.ReceiveTick`
  (params (DeltaSeconds :type "Float (single-precision)"))
  (bind (_returnvalue_x _returnvalue_y _returnvalue_z) (`KismetMathLibrary.BreakVector` (`SceneComponent.K2_GetComponentLocation` (`self.Sprite`))))
  (if (and (`self.Chasing`) (not (`self.RecievingDamage`)))
    (bind _asbp_rtv_game_character (cast `/Game/Actors/Blueprints/BP_RTV_GameCharacter` (`BlackboardComponent.GetValueAsObject` (`AIBlueprintHelperLibrary.GetBlackboard` self) "TargetedActor")))
    (if (>= (`self.GetDistanceTo` _asbp_rtv_game_character) 55.0)
      (set `self.Attacking` false)
      (bind (_returnvalue_x_2 _returnvalue_y_2) (`KismetMathLibrary.BreakVector` (`SceneComponent.K2_GetComponentLocation` (`PaperCharacter.Sprite` _asbp_rtv_game_character))))
      (`|AIMoveTo` (`self.GetController`) null (+ (`KismetMathLibrary.MakeVector` 0.0 _returnvalue_y_2) (`KismetMathLibrary.MakeVector` _returnvalue_x 0.0 _returnvalue_z)) null (`KismetMathLibrary.RandomFloatInRange` 0.0 50.0)
        (:`OnSuccess`
          (set `self.Attacking` true))))))

(event `OnDamaged`
  (params (Damage :type "Float (double-precision)") (DamageCauser :type "Actor Object Reference"))
  (bind _asbp_basic_enemy (cast `/Game/Actors/Enemy/BasicEnemy/Blueprints/BP_BasicEnemy` self))
  (`/Game/Actors/Enemy/BasicEnemy/Blueprints/BP_BasicEnemy.Damage` _asbp_basic_enemy Damage DamageCauser))

(event `Chase`
  (set `self.Chasing` true))

(event `SetAlerted`
  (set `self.Alerted` true)
  (`KismetSystemLibrary.Delay` 0.8)
  (set `self.Alerted` false))

(fn `Died`
  (`self.K2_DestroyActor`))

(fn `GetDirectionOppositeTarget`
  (params (Target :type "/Game/Actors/Player/Character/Blueprints/ND_PlayerSprite Object Reference"))
  (returns (Direction :type "/Game/Actors/Player/Character/Blueprints/ND_PlayerDirection Enum"))
  (bind _defaultplayerdirection (`/Game/Actors/Player/Character/Blueprints/ND_PlayerSprite.DefaultPlayerDirection` Target))
  (return (select `/Game/Actors/Player/Character/Blueprints/ND_PlayerDirection` (`/Game/Actors/Player/Character/Blueprints/ND_PlayerSprite.CurrentPlayerDirection` Target) :`NewEnumerator0` "NewEnumerator1" :`NewEnumerator1` "NewEnumerator0" :`NewEnumerator8` _defaultplayerdirection :`NewEnumerator9` _defaultplayerdirection :`NewEnumerator14` "NewEnumerator1" :`NewEnumerator15` "NewEnumerator0" :`NewEnumerator16` "NewEnumerator1" :`NewEnumerator17` "NewEnumerator0")))

(fn `SetActionState`
  (params (HorizontalVelocity :type "Float (double-precision)"))
  (returns (CurrentActionState :type "/Game/Actors/Enemy/Blueprints/E_EnemyState Enum") (NextActionState :type "/Game/Actors/Enemy/Blueprints/E_EnemyState Enum"))
  (bind _output_get (set `self.CurrentActionState` (`self.NextActionState`)))
  (bind _output_get_2 (set `self.NextActionState` (select `bool` (<= (`self.EnemyHealth`) 0.0) :`false` (select `bool` (`self.Alerted`) :`false` (select `bool` (`self.Attacking`) :`false` (select `bool` (!= HorizontalVelocity 0.0) :`false` "NewEnumerator0" :`true` "NewEnumerator1" :!type "/Game/Actors/Enemy/Blueprints/E_EnemyState Enum") :`true` "NewEnumerator2") :`true` "NewEnumerator3") :`true` "NewEnumerator4")))
  (return _output_get _output_get_2))

(fn `UserConstructionScript`
  (bind _capsulecomponent (`self.CapsuleComponent`))
  (set `self.HitBox` (make `/Game/Actors/Blueprints/HitBox` (`CapsuleComponent.CapsuleRadius` _capsulecomponent) (`CapsuleComponent.CapsuleHalfHeight` _capsulecomponent))))