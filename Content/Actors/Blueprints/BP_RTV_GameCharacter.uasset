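; Base 2D game character on the Y/Z plane, with melee attack, damage, knockback and movement-state helpers.
; Attack sphere-traces nearby pawns and runs sprite socket positions through a point-in-box test, but damages the character regardless of the result.
; Damaged forwards to OnDamaged only on ND_PlayerSprite instances.
; Helpers resolve eight-way dash facing, launch left/right knockback, clamp health and detect air or falling states.
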(event `self.ReceiveTick`
  (params (DeltaSeconds :type "Float (single-precision)")))

(event `Damaged`
  (params (DamageValue :type "Float (double-precision)") (DamageCauser :type "/Game/Actors/Blueprints/BP_RTV_GameCharacter Object Reference"))
  (bind _asnd_player_sprite (cast `/Game/Actors/Player/Character/Blueprints/ND_PlayerSprite` self))
  (`/Game/Actors/Player/Character/Blueprints/ND_PlayerSprite.OnDamaged` _asnd_player_sprite DamageValue DamageCauser))

(fn `ApplyDamage`
  (params (CurrentHealth :type "Float (double-precision)") (DamageAmount :type "Float (double-precision)") (MaxHealth :type "Float (double-precision)"))
  (returns (ResultingHealth :type "Float (double-precision)"))
  (return (`KismetMathLibrary.FClamp` (- CurrentHealth DamageAmount) 0.0 MaxHealth)))

(fn `Attack`
  (locals (HitDetect :type Boolean) (DetectPointLocationY :type "Float (double-precision)") (DetectPointLocationZ :type "Float (double-precision)") (EnemyLocationY :type "Float (double-precision)") (EnemyLocationZ :type "Float (double-precision)") (EnemyHitBoxHalfWidth :type "Float (double-precision)") (EnemyHitBoxHalfHeight :type "Float (double-precision)") (EnemyHitBoxWidth :type "Float (double-precision)") (EnemyHitBoxHeight :type "Float (double-precision)") (test :type Integer))
  (bind _sprite (`self.Sprite`))
  (bind _returnvalue (`SceneComponent.K2_GetComponentLocation` (`self.Sprite`)))
  (bind (_returnvalue_x _returnvalue_y _returnvalue_z) (`KismetMathLibrary.BreakVector` (`SceneComponent.K2_GetComponentLocation` _sprite)))
  (if (not (`self.HitDetected`))
    (bind _outhits (`KismetSystemLibrary.SphereTraceMultiForObjects` _returnvalue _returnvalue 90.0 (`|MakeArray` "ObjectTypeQuery3" :!type "EObjectTypeQuery Enum")))
    (for _array_element (`SceneComponent.GetAllSocketNames` _sprite)
      (if (stale _output_get_5)
        (break)
        (else
          (bind (_returnvalue_x_2 _returnvalue_y_2 _returnvalue_z_2) (`KismetMathLibrary.BreakVector` (`SceneComponent.GetSocketLocation` _sprite _array_element)))
          (set `local.DetectPointLocationY` _returnvalue_y_2)
          (set `local.DetectPointLocationZ` _returnvalue_z_2)
          (if (!= (`KismetMathLibrary.MakeVector` 0.0 _returnvalue_y_2 _returnvalue_z_2) (`KismetMathLibrary.MakeVector` 0.0 _returnvalue_y _returnvalue_z) :`ErrorTolerance` 0.001)
            (for _array_element_2 _outhits
              (bind _asbp_rtv_game_character (cast `/Game/Actors/Blueprints/BP_RTV_GameCharacter` (`.HitActor` (`GameplayStatics.BreakHitResult` _array_element_2))))
              (bind (_hitbox_halfwidth _hitbox_halfheight) (break `/Game/Actors/Blueprints/HitBox` (`/Game/Actors/Blueprints/BP_RTV_GameCharacter.HitBox` _asbp_rtv_game_character)))
              (bind _output_get (set `local.EnemyHitBoxHalfWidth` _hitbox_halfwidth))
              (bind _output_get_2 (set `local.EnemyHitBoxHalfHeight` _hitbox_halfheight))
              (bind (_returnvalue_x_3 _returnvalue_y_3 _returnvalue_z_3) (`KismetMathLibrary.BreakVector` (`SceneComponent.K2_GetComponentLocation` (`PaperCharacter.Sprite` _asbp_rtv_game_character))))
              (set `local.EnemyLocationY` _returnvalue_y_3)
              (set `local.EnemyLocationZ` _returnvalue_z_3)
              (bind _output_get_3 (set `local.EnemyHitBoxWidth` (* _output_get 2.0)))
              (bind _output_get_4 (set `local.EnemyHitBoxHeight` (* _output_get_2 2.0)))
              (`self.PointCollideHitbox` (`local.DetectPointLocationY`) (`local.DetectPointLocationZ`) (`local.EnemyLocationY`) (`local.EnemyLocationZ`) (`local.EnemyHitBoxHalfWidth`) (`local.EnemyHitBoxHalfHeight`) _output_get_3 _output_get_4)
              (bind _output_get_5 (set `self.HitDetected` true))
              (if true
                (`self.Damaged` _asbp_rtv_game_character (`self.BasicAttackDamage`) self)))))))))

(fn `DamageKnockback`
  (params (CharacterDirection :type "/Game/Actors/Player/Character/Blueprints/ND_PlayerDirection Enum" :default "NewEnumerator0") (Knockback :type "Float (double-precision)"))
  (`self.LaunchCharacter` (select `/Game/Actors/Player/Character/Blueprints/ND_PlayerDirection` CharacterDirection :`NewEnumerator0` (* (0.0 -300.0 300.0) Knockback) :`NewEnumerator1` (* (0.0 300.0 300.0) Knockback)) true true))

(fn `GetDirection`
  (params (LeftOrRight :type "Float (double-precision)") (UpOrDown :type "Float (double-precision)") (DefaultDirection :type "/Game/Actors/Player/Character/Blueprints/ND_PlayerDirection Enum" :default "NewEnumerator0") (Dashing :type Boolean))
  (returns (NextDirection :type "/Game/Actors/Player/Character/Blueprints/ND_PlayerDirection Enum"))
  (locals (LocalLeftOrRight :type "Float (double-precision)") (LocalUpOrDown :type "Float (double-precision)") (NextBaseDirection :type "/Game/Actors/Player/Character/Blueprints/ND_PlayerDirection Enum") (LocalDashing :type Boolean))
  (set `local.LocalLeftOrRight` LeftOrRight)
  (set `local.LocalUpOrDown` UpOrDown)
  (set `local.LocalDashing` Dashing)
  (if (`self.RecievingDamage`)
    (bind _output_get (set `local.NextBaseDirection` (`self.KnockbackFacingDirection`)))
    (return _output_get)
    (else
      (bind _output_get_2 (set `local.NextBaseDirection` (select `bool` (and (< (`local.LocalLeftOrRight`) 0.0) (> (`local.LocalUpOrDown`) 0.0) (`local.LocalDashing`)) :`false` (select `bool` (and (> (`local.LocalLeftOrRight`) 0.0) (> (`local.LocalUpOrDown`) 0.0) (`local.LocalDashing`)) :`false` (select `bool` (and (< (`local.LocalLeftOrRight`) 0.0) (< (`local.LocalUpOrDown`) 0.0) (`local.LocalDashing`)) :`false` (select `bool` (and (> (`local.LocalLeftOrRight`) 0.0) (< (`local.LocalUpOrDown`) 0.0) (`local.LocalDashing`)) :`false` (select `bool` (and (== (`local.LocalLeftOrRight`) 0.0) (> (`local.LocalUpOrDown`) 0.0) (`local.LocalDashing`)) :`false` (select `bool` (and (== (`local.LocalLeftOrRight`) 0.0) (< (`local.LocalUpOrDown`) 0.0) (`local.LocalDashing`)) :`false` (select `bool` (< (`local.LocalLeftOrRight`) 0.0) :`false` (select `bool` (> (`local.LocalLeftOrRight`) 0.0) :`false` DefaultDirection :`true` "NewEnumerator0") :`true` "NewEnumerator1") :`true` "NewEnumerator9") :`true` "NewEnumerator8") :`true` "NewEnumerator16") :`true` "NewEnumerator17") :`true` "NewEnumerator14") :`true` "NewEnumerator15")))
      (return _output_get_2))))

(fn `IsFalling`
  (params (VerticalVelocity :type "Float (double-precision)"))
  (returns (IsFalling :type Boolean))
  (return (< VerticalVelocity -58.0)))

(fn `IsInAir`
  (returns (IsInAir :type Boolean))
  (bind (_hitbox_halfwidth _hitbox_halfheight) (break `/Game/Actors/Blueprints/HitBox` (`self.HitBox`)))
  (bind _returnvalue (`self.K2_GetActorLocation` self))
  (bind _outhit (`KismetSystemLibrary.CapsuleTraceSingleForObjects` :`Start` _returnvalue :`End` (+ _returnvalue (0.0 0.0 -999999995904.0)) :`Radius` _hitbox_halfwidth :`HalfHeight` _hitbox_halfheight :`ObjectTypes` (`|MakeArray` "ObjectTypeQuery1" "ObjectTypeQuery2" "ObjectTypeQuery4" :!type "EObjectTypeQuery Enum") :`DrawDebugType` "ForOneFrame"))
  (if (> (`.Distance` (`GameplayStatics.BreakHitResult` _outhit)) 2.2)
    (return true)
    (else
      (return false))))

(fn `PointCollideHitbox`
  (params (PointLocationY :type "Float (double-precision)") (PointLocationZ :type "Float (double-precision)") (HitBoxCenterLocationY :type "Float (double-precision)") (HitBoxCenterLocationZ :type "Float (double-precision)") (HitBoxHalfWidth :type "Float (double-precision)") (HitBoxHalfHeight :type "Float (double-precision)") (HitBoxWidth :type "Float (double-precision)") (HitBoxHeight :type "Float (double-precision)"))
  (returns (Collision :type Boolean))
  (return (and (<= (- (+ HitBoxCenterLocationY HitBoxHalfWidth) PointLocationY) HitBoxWidth) (<= (- (+ HitBoxCenterLocationZ HitBoxHalfHeight) PointLocationZ) HitBoxHeight) (<= (- PointLocationY (- HitBoxCenterLocationY HitBoxHalfWidth)) HitBoxWidth) (<= (- PointLocationZ (- HitBoxCenterLocationZ HitBoxHalfHeight)) HitBoxHeight))))

(fn `UserConstructionScript`)