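; BP_MainCharacter is the player's 2D flipbook character, with side-on movement along Y, jumping and an eight-way dash.
; Dash snapshots input axes, defaulting to facing direction, launches the character, then after a brief delay relaunches at a small fraction of that velocity to brake.
; Each Tick detects falling from Z velocity, then Animate picks a flipbook by facing and a prioritized action state: dash, jump, fall, attack, move, idle.
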(event `self.ReceiveTick`
  (params (DeltaSeconds :type "Float (single-precision)"))
  (bind (_returnvalue_x _returnvalue_y _returnvalue_z) (`KismetMathLibrary.BreakVector` (`self.GetVelocity`)))
  (if (and (< _returnvalue_z -58.0) (not (`self.Dashing`)))
    (set `self.Falling` true)
    (set `self.Jumping` false)
    (else
      (set `self.Falling` false)))
  (`self.Animate`))

(event `InputAxis|LeftOrRight`
  (params (AxisValue :type "Float (single-precision)"))
  (`self.AddMovementInput` (0.0 -1.0 0.0) AxisValue))

(event `InputAction|Jump`
  (params (Key :type "Key Structure"))
  (:`Pressed`
    (set `self.Jumping` true)
    (`self.Jump`)))

(event `InputAction|Dash`
  (params (Key :type "Key Structure"))
  (:`Pressed`
    (set `self.Dash Direction Left or Right` (`self.GetInputAxisValue`))
    (set `self.Dash Direction Up or Down` (`self.GetInputAxisValue`))
    (set `self.Dashing` true)
    (set `self.Jumping` false)
    (bind _dashdirection (`self.GetDashDirection`))
    (bind _returnvalue (select `/Game/Assets/Player/Character/Blueprints/E_PlayerDirection` _dashdirection :`NewEnumerator0` (0.0 0.0 3000.0) :`NewEnumerator1` (0.0 0.0 -3000.0) :`NewEnumerator2` (0.0 3000.0 0.0) :`NewEnumerator3` (0.0 -3000.0 0.0) :`NewEnumerator4` (0.0 2121.320312 2121.320312) :`NewEnumerator5` (0.0 -2121.320312 2121.320312) :`NewEnumerator6` (0.0 2121.320312 -2121.320312) :`NewEnumerator7` (0.0 -2121.320312 -2121.320312) :!type "Vector Structure"))
    (`self.LaunchCharacter` _returnvalue true true)
    (`KismetSystemLibrary.Delay` 0.1)
    (`self.LaunchCharacter` (* _returnvalue (0.033333 0.033333 0.033333)) true true)
    (set `self.Dashing` false)))

(fn `Animate`
  (set `self.LocalLeftOrRight` (`self.GetInputAxisValue`))
  (`self.SetAction`)
  ;[1 1 1] Check Facing Direction
  (if (> (`self.GetInputAxisValue`) 0.0)
    (set `self.FacingRIght` true))
  (if (< (`self.GetInputAxisValue`) 0.0)
    (set `self.FacingRIght` false))
  (`PaperFlipbookComponent.SetFlipbook` (`self.Sprite`) (select `bool` (`self.FacingRIght`) :`false` (select `byte` (`self.NextActionState`) :`0` null :`1` null :`2` null :`3` null :`4` null :`5` null :`6` null :!type "PaperFlipbook Object Reference") :`true` (select `byte` (`self.NextActionState`) :`0` null :`1` null :`2` null :`3` null :`4` null :`5` null :`6` null :!type "PaperFlipbook Object Reference"))))

(fn `GetDashDirection`
  (returns (DashDirection :type "/Game/Assets/Player/Character/Blueprints/E_PlayerDirection Enum"))
  (if (> (`self.Dash Direction Left or Right`) 0.0)
    ;[1 1 1] Right
    (return (select `bool` (> (`self.Dash Direction Up or Down`) 0.0) :`false` (select `bool` (< (`self.Dash Direction Up or Down`) 0.0) :`false` "NewEnumerator3" :`true` "NewEnumerator7" :!type "/Game/Assets/Player/Character/Blueprints/E_PlayerDirection Enum") :`true` "NewEnumerator5"))
    (elif (< (`self.Dash Direction Left or Right`) 0.0)
      ;[1 1 1] Left
      (return (select `bool` (> (`self.Dash Direction Up or Down`) 0.0) :`false` (select `bool` (< (`self.Dash Direction Up or Down`) 0.0) :`false` "NewEnumerator2" :`true` "NewEnumerator6" :!type "/Game/Assets/Player/Character/Blueprints/E_PlayerDirection Enum") :`true` "NewEnumerator4"))
      (else
        ;[1 1 1] Up/Down
        (return (select `bool` (> (`self.Dash Direction Up or Down`) 0.0) :`false` (select `bool` (< (`self.Dash Direction Up or Down`) 0.0) :`false` (select `bool` (`self.FacingRIght`) :`false` "NewEnumerator2" :`true` "NewEnumerator3" :!type "/Game/Assets/Player/Character/Blueprints/E_PlayerDirection Enum") :`true` "NewEnumerator1") :`true` "NewEnumerator0"))))))

(fn `SetAction`
  (set `self.NextActionState` (select `bool` (`self.Dashing`) :`false` (select `bool` (`self.Jumping`) :`false` (select `bool` (`self.Falling`) :`false` (select `bool` (`self.Attacking`) :`false` (select `bool` (!= (`self.LocalLeftOrRight`) 0.0) :`false` "NewEnumerator0" :`true` "NewEnumerator6" :!type "/Game/Assets/Player/Character/Blueprints/E_PlayerState Enum") :`true` "NewEnumerator12") :`true` "NewEnumerator16") :`true` "NewEnumerator10") :`true` "NewEnumerator8")))

(fn `UserConstructionScript`)