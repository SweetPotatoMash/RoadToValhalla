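; BP_RTV_GameCharacter is a game character Blueprint whose only logic is a 2D hitbox test; its events and construction script are empty.
; PointCollideHitbox reports whether a point lies within an axis-aligned box on the Y/Z plane, using plain arithmetic rather than engine collision.
; It compares the point's distance from each box edge against the full width or height, with half and full sizes supplied by the caller.
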(fn `PointCollideHitbox`
  (params (PointLocationY :type "Float (double-precision)") (PointLocationZ :type "Float (double-precision)") (HitBoxCenterLocationY :type "Float (double-precision)") (HitBoxCenterLocationZ :type "Float (double-precision)") (HitBoxHalfWidth :type "Float (double-precision)") (HitBoxHalfHeight :type "Float (double-precision)") (HitBoxWidth :type "Float (double-precision)") (HitBoxHeight :type "Float (double-precision)"))
  (returns (Collision :type Boolean))
  (return (and (<= (- (+ HitBoxCenterLocationY HitBoxHalfWidth) PointLocationY) HitBoxWidth) (<= (- (+ HitBoxCenterLocationZ HitBoxHalfHeight) PointLocationZ) HitBoxHeight) (<= (- PointLocationY (- HitBoxCenterLocationY HitBoxHalfWidth)) HitBoxWidth) (<= (- PointLocationZ (- HitBoxCenterLocationZ HitBoxHalfHeight)) HitBoxHeight))))

(fn `UserConstructionScript`)